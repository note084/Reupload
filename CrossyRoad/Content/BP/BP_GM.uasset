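; BP_GM is the game manager and auto-scrolling camera for a chicken game, tracking score, high score and coins.
; It makes itself the view target and advances along X until the chicken is hit, spawning a single eagle if the chicken leaves the screen.
; Increment functions update the score widget it creates.
; The high score loads from a save slot in the construction script and saves on EndPlay.
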(event `self.ReceiveBeginPlay`
  (bind _returnvalue (`|CreateWidget` "/Game/UI/Widget_Scores.Widget_Scores_C"))
  (`UserWidget.AddToViewport` _returnvalue 0)
  (set `/Game/UI/Widget_Scores.GameManager` self _returnvalue)
  (set `self.SW` _returnvalue)
  (set `self.bFindCameraComponentWhenViewTarget` true)
  (`PlayerController.SetViewTargetWithBlend` (`GameplayStatics.GetPlayerController` 0) self 0.0 "VTBlend_Linear" 0.0 false)
  (bind _outactors (`GameplayStatics.GetAllActorsOfClass` "/Game/Chicken_Assets/BP_Chicken.BP_Chicken_C"))
  (set `self.Player` (`|GetArrayItem` _outactors))
  (`/Game/UI/Widget_Scores.UpdateTopScore` (`self.SW`)))

(event `self.ReceiveTick`
  (params (DeltaSeconds :type "Float (single-precision)"))
  (if (not (`/Game/Chicken_Assets/BP_Chicken.Hit` (`self.Player`)))
    (`self.AddMovementInput` (0.7 0.0 0.0) 100.0)
    (bind _returnvalue (`self.ConsumeMovementInputVector`))
    (`self.K2_AddActorLocalOffset` (* _returnvalue DeltaSeconds) true)
    (`self.CheckPlayer`)))

(event `self.ReceiveEndPlay`
  (params (EndPlayReason :type "EEndPlayReason Enum" :default "Destroyed"))
  (bind _save (`self.Save`))
  (set `/Game/BP/BP_HighScore.HS` (`self.HS`) _save)
  (`GameplayStatics.SaveGameToSlot` _save (`/Game/BP/BP_HighScore.SAVE` _save))
  (`KismetSystemLibrary.PrintString` "Saved game data" false false))

(fn `CheckPlayer`
  (bind (_returnvalue_x _returnvalue_y _returnvalue_z) (`KismetMathLibrary.BreakVector` (`self.K2_GetActorLocation` (`self.Player`))))
  (if (`.ReturnValue` (`GameplayStatics.ProjectWorldToScreen` (`GameplayStatics.GetPlayerController` 0) (`self.K2_GetActorLocation` (`self.Player`)) true))
    _
    (elif (not (`self.Eagle`))
      (bind _returnvalue (`|SpawnActorFromClass` "/Game/Game_Assets/Eagle/BP_Eagle.BP_Eagle_C" (`KismetMathLibrary.MakeTransform` (`KismetMathLibrary.MakeVector` (+ _returnvalue_x 800.0) _returnvalue_y (+ _returnvalue_z 100.0))) "Undefined" "OverrideRootScale" null null))
      (set `/Game/Game_Assets/Eagle/BP_Eagle.Player` (`self.Player`) _returnvalue)
      (set `self.Eagle` true))))

(fn `IncrementCoins`
  (`/Engine/EditorBlueprintResources/StandardMacros.IncrementInt` (`self.CC`)
    (:`  `
      (`/Game/UI/Widget_Scores.UpdateCoinCounter` (`self.SW`)))))

(fn `IncrementScore`
  (bind _output_get (set `self.S` (+ (`self.S`) 1)))
  (`/Game/UI/Widget_Scores.UpdateScoreCounter` (`self.SW`))
  (if (> _output_get (`self.HS`))
    (set `self.HS` (`self.S`))
    (`/Game/UI/Widget_Scores.UpdateTopScore` (`self.SW`))))

(fn `UserConstructionScript`
  (bind _returnvalue (`GameplayStatics.CreateSaveGameObject` "/Game/BP/BP_HighScore.BP_HighScore_C"))
  (bind _output_get (set `self.Save` _returnvalue))
  (bind _returnvalue_2 (`GameplayStatics.LoadGameFromSlot` (`/Game/BP/BP_HighScore.SAVE` _output_get)))
  (bind _asbp_high_score (cast `/Game/BP/BP_HighScore` _returnvalue_2))
  (bind _output_get_2 (set `self.Save` _asbp_high_score))
  (set `self.HS` (`/Game/BP/BP_HighScore.HS` _output_get_2))
  (`KismetSystemLibrary.PrintString` "Loaded game data" false false))